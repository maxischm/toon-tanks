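; Game mode Blueprint for Toon Tanks that shows the UI for game start, new waves and game over.
; Each event creates its own widget and adds it to the viewport.
; Game over sets win or lose text from the WonGame flag.
; New waves display the wave number, then remove that widget after a short delay.
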(event EventBeginPlay)

(event EventTick
  (params (DeltaSeconds :type Float%20%28single-precision%29)))

(event EventStartGame
  (bind _returnvalue (UserInterface|CreateWidget "/Game/Blueprints/Widgets/WBP_StartGameWidget.WBP_StartGameWidget_C"))
  (UserInterface|Viewport|AddtoViewport _returnvalue 0))

(event EventGameOver
  (params (bWonGame :type Boolean))
  (bind _returnvalue (UserInterface|CreateWidget "/Game/Blueprints/Widgets/WBP_EndGameWidget.WBP_EndGameWidget_C"))
  (UserInterface|Viewport|AddtoViewport _returnvalue 0)
  (Rendering|Components|TextRender|SetText (Variables|/Game/Blueprints/Widgets/WBP_EndGameWidget.WBP_EndGameWidget_C|GetDisplayText _returnvalue) (select bWonGame "YOU WON!" "YOU LOST!")))

(event EventNewWave
  (params (WaveNumber :type Integer))
  (bind _returnvalue (UserInterface|CreateWidget "/Game/Blueprints/Widgets/WBP_NewWaveWidget.WBP_NewWaveWidget_C"))
  (UserInterface|Viewport|AddtoViewport _returnvalue 0)
  (Rendering|Components|TextRender|SetText (Variables|/Game/Blueprints/Widgets/WBP_NewWaveWidget.WBP_NewWaveWidget_C|GetWaveNumberText _returnvalue) (Utilities|Text|ToText(String) (Utilities|String|Append (Utilities|String|MakeLiteralString "Wave ") (Utilities|String|ToString(Integer) WaveNumber))))
  (Utilities|FlowControl|Delay 2.0)
  (Widget|RemovefromParent _returnvalue))

(fn ConstructionScript)